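; Player controller that maps desktop and VR input to BP_VPPlayerPawn actions: movement, look, teleport, gizmo interaction, pickup, tool change and context menu.
; BeginPlay caches the pawn and sets the temporary player state that gates teleport and zoom axes.
; Several actions also feed press/release to a meta-input interpreter, and a focus event feeds another.
; Pickup and tool selection toggle through booleans; threshold initialization and SubFunction press/release logic are disconnected.
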(event Custom|InputMetadata%20Init%20이벤트
  (bind _editoractionmetainputinterpreter (Variables|Default|GetEditorActionMetaInputInterpreter))
  (bind _editorfocusmetainputinterpreter (Variables|Default|GetEditorFocusMetaInputInterpreter))
  ;[1 1 1] 사용자 메타데이터 입력값 초기화
  (Utilities|FlowControl|Sequence
    (:then_0
      (Utilities|FlowControl|Sequence
        (:then_0
          (Variables|/Script/UEPrototype.EditorActionMetaInputInterpreter|SetTriggerThreshold _editoractionmetainputinterpreter 0.12))
        (:then_1
          (Variables|/Script/UEPrototype.EditorActionMetaInputInterpreter|SetClickThreshold _editoractionmetainputinterpreter 0.4))))
    (:then_1
      (Utilities|FlowControl|Sequence
        (:then_0
          (Variables|/Script/UEPrototype.EditorFocusMetaInputInterpreter|SetFocusTime _editorfocusmetainputinterpreter 0.0))
        (:then_1
          (Variables|/Script/UEPrototype.EditorFocusMetaInputInterpreter|SetTimeToHighlight _editorfocusmetainputinterpreter 1.0))))))

(event Custom|SetSubFunction_EXP
  ;[0 8 10] 일반 : SubFunction 입력 / 컨텍스트 메뉴 호출 (우클릭)
  (Variables|Default|SetbSubFunction (Game|Player|WasInputKeyJustPressed (Game|GetPlayerController 0) "L")))

(event EventTick
  (params (DeltaSeconds :type Float%20%28single-precision%29))
  (CallFunction|SetSubFunctionEXP))

(event EventBeginPlay
  ;[1 1 1] 블루프린트 변수 초기화
  (Utilities|FlowControl|Sequence
    (:then_0
      (Variables|Default|SetPPlayerTempState "NewEnumerator2"))
    (:then_1
      (bind _asbp_vpplayer_pawn (Utilities|Casting|CastToBP_VPPlayerPawn (Pawn|GetControlledPawn)))
      (Variables|Core|Player|SetVPDirectorPawn _asbp_vpplayer_pawn))))

(event EventFocusEvent
  (params (Target :type Actor%20Object%20Reference) (DeltaTime :type Float%20%28single-precision%29))
  (bind _editorfocusmetainputinterpreter (Variables|Default|GetEditorFocusMetaInputInterpreter))
  ;[20 10 0] Focus 이벤트(매 Tick마다 호출)
  (Utilities|IsValid _editorfocusmetainputinterpreter
    (:Is%20Valid
      (Class|EditorFocusMetaInputInterpreter|InterpreteFocus _editorfocusmetainputinterpreter Target DeltaTime))))

(event Input|ActionEvents|InputActionMainFunction
  (params (Key :type Key%20Structure))
  (bind _editoractionmetainputinterpreter (Variables|Default|GetEditorActionMetaInputInterpreter))
  ;[0 8 10] 일반 : MainFunction 입력 / 액터 및 위젯 상호작용 (좌클릭)
  (:Pressed
    (Class|EditorActionMetaInputInterpreter|ReceivePressed _editoractionmetainputinterpreter "MainFunction")
    (Default|GizmoInteraction (Variables|Core|Player|GetVPDirectorPawn)))
  (:Released
    (Class|EditorActionMetaInputInterpreter|ReceiveReleased _editoractionmetainputinterpreter "MainFunction")))

(event Input|ActionEvents|InputActionCallMenu
  (params (Key :type Key%20Structure))
  (bind _editoractionmetainputinterpreter (Variables|Default|GetEditorActionMetaInputInterpreter))
  ;[0 8 10] 일반 : 도구 메뉴창 입력 (D)
  (:Pressed
    (Class|EditorActionMetaInputInterpreter|ReceivePressed _editoractionmetainputinterpreter "CallMenu"))
  (:Released
    (Class|EditorActionMetaInputInterpreter|ReceiveReleased _editoractionmetainputinterpreter "CallMenu")))

(event Input|ActionEvents|InputActionSubFunction
  (params (Key :type Key%20Structure))
  ;[0 8 10] 일반 : SubFunction 입력 / 컨텍스트 메뉴 호출 (우클릭)
)

(event Input|ActionEvents|InputActionGizmoTestMode
  (params (Key :type Key%20Structure))
  (:Pressed
    (Default|GizmoModeChange (Variables|Core|Player|GetVPDirectorPawn))))

(event Input|ActionEvents|InputActionCancel
  (params (Key :type Key%20Structure))
  (bind _editoractionmetainputinterpreter (Variables|Default|GetEditorActionMetaInputInterpreter))
  ;[0 8 10] 일반 : Cancel 입력 (Esc)
  (:Pressed
    (Class|EditorActionMetaInputInterpreter|ReceivePressed _editoractionmetainputinterpreter "Cancel")
    (if (Utilities|Enum|Equal(Enum) (Variables|Default|GetPPlayerTempState) "NewEnumerator0")
      _))
  (:Released
    (Class|EditorActionMetaInputInterpreter|ReceiveReleased _editoractionmetainputinterpreter "Cancel")))

(event Input|ActionEvents|InputActionGizmoTestCoord
  (params (Key :type Key%20Structure))
  (:Pressed
    (Default|GizmoCoordinateChange (Variables|Core|Player|GetVPDirectorPawn))))

(event Input|ActionEvents|InputActionTeleport
  (params (Key :type Key%20Structure))
  (bind _editoractionmetainputinterpreter (Variables|Default|GetEditorActionMetaInputInterpreter))
  ;[1.006 10 0] 이동 : Teleport 입력 (T)
  (:Pressed
    (Class|EditorActionMetaInputInterpreter|ReceivePressed _editoractionmetainputinterpreter "Teleport")
    (if (Utilities|Enum|Equal(Enum) (Variables|Default|GetPPlayerTempState) "NewEnumerator2")
      (Default|Teleport (Variables|Core|Player|GetVPDirectorPawn))))
  (:Released
    (Class|EditorActionMetaInputInterpreter|ReceiveReleased _editoractionmetainputinterpreter "Teleport")))

(event Input|ActionEvents|InputActionPick
  (params (Key :type Key%20Structure))
  (bind _editoractionmetainputinterpreter (Variables|Default|GetEditorActionMetaInputInterpreter))
  (bind _vpdirectorpawn (Variables|Core|Player|GetVPDirectorPawn))
  ;[1 2 1] 트랜스폼 : Pickup 입력 (MMB)
  (:Pressed
    (Class|EditorActionMetaInputInterpreter|ReceivePressed _editoractionmetainputinterpreter "Pick")
    (if (Variables|Default|GetbCanPick)
      (Default|PickUp _vpdirectorpawn)
      (Variables|Default|SetbCanPick false)
      (else
        (Default|Drop _vpdirectorpawn)
        (Variables|Default|SetbCanPick true))))
  (:Released
    (Class|EditorActionMetaInputInterpreter|ReceiveReleased _editoractionmetainputinterpreter "Pick")))

(event Input|AxisEvents|InputAxisZoomPickup
  (params (AxisValue :type Float%20%28single-precision%29))
  ;[1 2 1] 트랜스폼 : ZoomPickup 축 (MMB Wheel)
  (if (Utilities|Enum|Equal(Enum) (Variables|Default|GetPPlayerTempState) "NewEnumerator1")
    (Default|ZoomPickupPoint (Variables|Core|Player|GetVPDirectorPawn) AxisValue 5.0)))

(event Input|AxisEvents|InputAxisMoveRight
  (params (AxisValue :type Float%20%28single-precision%29))
  ;[20 10 0] 이동(VR : XY 지원, 데스크탑 : XYZ 지원)
  (Class|VPDirectorPawn|MoveAround (Variables|Core|Player|GetVPDirectorPawn) "MT_LOCALAXIS" (stale Input|AxisEvents|InputAxisMoveForward AxisValue) AxisValue (stale Input|AxisEvents|InputAxisMoveUp AxisValue) 0))

(event Input|AxisEvents|InputAxisMoveForward
  (params (AxisValue :type Float%20%28single-precision%29))
  ;[20 10 0] 이동(VR : XY 지원, 데스크탑 : XYZ 지원)
  (Class|VPDirectorPawn|MoveAround (Variables|Core|Player|GetVPDirectorPawn) "MT_LOCALAXIS" AxisValue (stale Input|AxisEvents|InputAxisMoveRight AxisValue) (stale Input|AxisEvents|InputAxisMoveUp AxisValue) 0))

(event Input|AxisEvents|InputAxisLookUp
  (params (AxisValue :type Float%20%28single-precision%29))
  ;[20 10 0] 회전 (데스크탑 전용)
  (Class|VPDirectorPawn|LookUpSide (Variables|Core|Player|GetVPDirectorPawn) AxisValue))

(event Input|AxisEvents|InputAxisLookSide
  (params (AxisValue :type Float%20%28single-precision%29))
  ;[20 10 0] 회전 (데스크탑 전용)
  (Class|VPDirectorPawn|LookSide (Variables|Core|Player|GetVPDirectorPawn) AxisValue))

(event Input|AxisEvents|InputAxisMoveUp
  (params (AxisValue :type Float%20%28single-precision%29))
  ;[20 10 0] 이동(VR : XY 지원, 데스크탑 : XYZ 지원)
  (Class|VPDirectorPawn|MoveAround (Variables|Core|Player|GetVPDirectorPawn) "MT_LOCALAXIS" (stale Input|AxisEvents|InputAxisMoveForward AxisValue) (stale Input|AxisEvents|InputAxisMoveRight AxisValue) AxisValue 0))

(event Input|AxisEvents|InputAxisZoomTeleport
  (params (AxisValue :type Float%20%28single-precision%29))
  (if (Utilities|Enum|Equal(Enum) (Variables|Default|GetPPlayerTempState) "NewEnumerator2")
    (Default|ZoomTeleportPoint (Variables|Core|Player|GetVPDirectorPawn) AxisValue 1e+02)))

(event Input|KeyboardEvents|MotionControllerLeftThumbstick
  (params (Key :type Key%20Structure))
  (bind _vpdirectorpawn (Variables|Core|Player|GetVPDirectorPawn))
  ;[1 2 1] 트랜스폼 : Pickup 입력 (MMB)
  (:Pressed
    (Class|EditorActionMetaInputInterpreter|ReceivePressed (Variables|Default|GetEditorActionMetaInputInterpreter) "Pick")
    (if (Variables|Default|GetbCanPick)
      (Default|PickUp _vpdirectorpawn)
      (Variables|Default|SetbCanPick false)
      (else
        (Default|Drop _vpdirectorpawn)
        (Variables|Default|SetbCanPick true)))))

(event Input|KeyboardEvents|MotionControllerRightFaceButton2
  (params (Key :type Key%20Structure))
  ;[1 1 1] 컨텍스트 창 띄우기
  (:Pressed
    (Default|ShowContext (Variables|Core|Player|GetVPDirectorPawn))))

(event Input|KeyboardEvents|MotionControllerRightThumbstick
  (params (Key :type Key%20Structure))
  (bind _vpdirectorpawn (Variables|Core|Player|GetVPDirectorPawn))
  (:Pressed
    (if (Variables|Default|GetbCanSelctTool)
      (Default|ChangeTool _vpdirectorpawn)
      (Variables|Default|SetbCanSelctTool false)
      (else
        (Default|EndChangeTool _vpdirectorpawn)
        (Variables|Default|SetbCanSelctTool true)))))

(event Input|KeyboardEvents|Y
  (params (Key :type Key%20Structure))
  (:Pressed
    ;[1 1 1] 컨텍스트 창 띄우기
    (Default|ShowContext (Variables|Core|Player|GetVPDirectorPawn))))

(fn ConstructionScript)